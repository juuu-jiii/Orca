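; BP_LEDPanel is an LED panel actor that cycles its chevron material through an array of colours once per second.
; BeginPlay creates a dynamic material instance on the panel mesh and sets its PanVelocity parameter from XVelocity.
; Tick accumulates elapsed time and calls ChangeMaterial, which advances the index with modulo wraparound and updates the instance's Colour parameter rather than swapping materials.
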(event `self.ReceiveBeginPlay`
  ;[1 1 1] Sets initial material based on materialIndex variable value.
  (bind _returnvalue (`PrimitiveComponent.CreateDynamicMaterialInstance` (`self.SM_LEDPanel`) 0 null "None")) ; Dynamic Material Instances allow for changes\nto be made to them during runtime. Returns a\nreference to the instance created.
  (bind _output_get (set `self.mat` _returnvalue)) ; Store reference to dynamic material\n (here of type M_Chevron) in a variable,\nso it can be accessed in ChangeMaterial().
  (`MaterialInstanceDynamic.SetVectorParameterValue` _output_get "PanVelocity" (`KismetMathLibrary.MakeColor` (`self.xVelocity`))) ; M_Chevron has a parameter called\nColour, which allows for changes to be\nmade to the material's colour via\nblueprints.
)

(event `self.ReceiveTick`
  (params (DeltaSeconds :type "Float (single-precision)"))
  ;[1 1 1] Calls ChangeMaterial() every second elapsed.
  (bind _output_get (set `self.elapsedTime` (+ DeltaSeconds (`self.elapsedTime`))))
  (if (>= _output_get 1.0)
    (set `self.elapsedTime` 0.0)
    (`self.ChangeMaterial`)))

(fn `ChangeMaterial`
  ;[1 1 1] Sets the current material to the next one in the materials array, wrapping around if the end is reached.
  (set `self.materialIndex` (mod (+ (`self.materialIndex`) 1) (`KismetArrayLibrary.Array_Length` (`self.colours`))))
  (`MaterialInstanceDynamic.SetVectorParameterValue` (`self.mat`) "Colour" (`KismetMathLibrary.Conv_VectorToLinearColor` (`|GetArrayItem` (`self.colours`) (`self.materialIndex`)))) ; Same as in Event Graph.
)

(fn `UserConstructionScript`)