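; Player pawn that drives itself forward once accelerated and turns in 90-degree yaw steps.
; Accelerate and Brake toggle a Moving flag; while it is set, Tick feeds forward movement input and the strafe axis adds right-plus-forward input.
; Steer Left and Right snap the actor rotation, and each Tick draws a debug forward line trace.
; Several unconnected movement, root-component and collision experiments remain in the event graph.
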(event `self.ReceiveBeginPlay`)

(event `self.ReceiveTick`
  (params (DeltaSeconds :type "Float (single-precision)"))
  (`self.ShowForwardVector`)
  (if (`self.moving`)
    (`self.AddMovementInput` (`self.GetActorForwardVector`))))

(event `InputAction|Accelerate`
  (params (Key :type "Key Structure"))
  (:`Pressed`
    (set `self.moving` true)))

(event `InputAction|Brake`
  (params (Key :type "Key Structure"))
  (:`Pressed`
    (set `self.moving` false)))

(event `InputAxis|Strafe Right`
  (params (AxisValue :type "Float (single-precision)"))
  (if (`self.moving`)
    (`self.AddMovementInput` (+ (* (`self.GetActorRightVector`) AxisValue) (`self.GetActorForwardVector`)))))

(event `InputAction|Steer Left`
  (params (Key :type "Key Structure"))
  (bind (_returnvalue_roll _returnvalue_pitch _returnvalue_yaw) (`KismetMathLibrary.BreakRotator` (`self.K2_GetActorRotation`)))
  (:`Pressed`
    (`self.K2_SetActorRotation` (`KismetMathLibrary.MakeRotator` 0.0 0.0 (+ -90.0 _returnvalue_yaw)))))

(event `InputAction|Steer Right`
  (params (Key :type "Key Structure"))
  (bind (_returnvalue_roll _returnvalue_pitch _returnvalue_yaw) (`KismetMathLibrary.BreakRotator` (`self.K2_GetActorRotation`)))
  (:`Pressed`
    (`self.K2_SetActorRotation` (`KismetMathLibrary.MakeRotator` 0.0 0.0 (+ 90.0 _returnvalue_yaw)))))

(fn `ShowForwardVector`
  (bind _returnvalue (`self.K2_GetActorLocation`))
  (`KismetSystemLibrary.LineTraceSingle` :`Start` _returnvalue :`End` (+ _returnvalue (* (`self.GetActorForwardVector`) 5000.0)) :`TraceChannel` "TraceTypeQuery1" :`DrawDebugType` "ForOneFrame"))

(fn `UserConstructionScript`)