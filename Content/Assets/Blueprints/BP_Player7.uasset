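; BP_Player7 is a player pawn that drives forward on its own after Accelerate until Brake is pressed.
; Tick feeds forward movement input while Moving, Strafe Right adds a combined forward and sideways vector, and Steer Left/Right snap yaw by 90 degrees.
; Collision handling is debug only: Box hits draw a point at impact, and front, left and right colliders print their side on hit or overlap.
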(event `InputAction|Accelerate`
  (params (Key :type "Key Structure"))
  (:`Pressed`
    (set `self.moving` true)))

(event `InputAction|Brake`
  (params (Key :type "Key Structure"))
  (:`Pressed`
    (set `self.moving` false)))

(event `self.ReceiveTick`
  (params (DeltaSeconds :type "Float (single-precision)"))
  (if (`self.moving`)
    (`self.AddMovementInput` (`self.GetActorForwardVector`))))

(event `InputAxis|Strafe Right`
  (params (AxisValue :type "Float (single-precision)"))
  (if (`self.moving`)
    (`self.AddMovementInput` (+ (* (`self.GetActorRightVector`) AxisValue) (`self.GetActorForwardVector`)) 10000.0)))

(event `InputAction|Steer Left`
  (params (Key :type "Key Structure"))
  (bind (_returnvalue_roll _returnvalue_pitch _returnvalue_yaw) (`KismetMathLibrary.BreakRotator` (`self.K2_GetActorRotation`)))
  (:`Pressed`
    (`self.K2_SetActorRotation` (`KismetMathLibrary.MakeRotator` 0.0 0.0 (+ -90.0 _returnvalue_yaw)))))

(event `InputAction|Steer Right`
  (params (Key :type "Key Structure"))
  (bind (_returnvalue_roll _returnvalue_pitch _returnvalue_yaw) (`KismetMathLibrary.BreakRotator` (`self.K2_GetActorRotation`)))
  (:`Pressed`
    (`self.K2_SetActorRotation` (`KismetMathLibrary.MakeRotator` 0.0 0.0 (+ 90.0 _returnvalue_yaw)))))

(event `self.Box.OnComponentBeginOverlap`
  (params (OverlappedComponent :type "PrimitiveComponent Object Reference") (OtherActor :type "Actor Object Reference") (OtherComp :type "PrimitiveComponent Object Reference") (OtherBodyIndex :type Integer) (bFromSweep :type Boolean) (SweepResult :type "HitResult Structure (by ref)")))

(event `self.Box.OnComponentHit`
  (params (HitComponent :type "PrimitiveComponent Object Reference") (OtherActor :type "Actor Object Reference") (OtherComp :type "PrimitiveComponent Object Reference") (NormalImpulse :type "Vector Structure") (Hit :type "HitResult Structure (by ref)"))
  (`KismetSystemLibrary.DrawDebugPoint` (`.ImpactPoint` (`GameplayStatics.BreakHitResult` Hit)) 100.0 (struct :`G` 1.0 :`B` 0.968645 :`A` 1.0) 1.0))

(event `self.Front Collider.OnComponentHit`
  (params (HitComponent :type "PrimitiveComponent Object Reference") (OtherActor :type "Actor Object Reference") (OtherComp :type "PrimitiveComponent Object Reference") (NormalImpulse :type "Vector Structure") (Hit :type "HitResult Structure (by ref)"))
  (`KismetSystemLibrary.PrintString` "front" :!label _label))

(event `self.Right Collider.OnComponentHit`
  (params (HitComponent :type "PrimitiveComponent Object Reference") (OtherActor :type "Actor Object Reference") (OtherComp :type "PrimitiveComponent Object Reference") (NormalImpulse :type "Vector Structure") (Hit :type "HitResult Structure (by ref)"))
  (`KismetSystemLibrary.PrintString` "right" :!label _label_2))

(event `self.Left Collider.OnComponentHit`
  (params (HitComponent :type "PrimitiveComponent Object Reference") (OtherActor :type "Actor Object Reference") (OtherComp :type "PrimitiveComponent Object Reference") (NormalImpulse :type "Vector Structure") (Hit :type "HitResult Structure (by ref)"))
  (`KismetSystemLibrary.PrintString` "left" :!label _label_3))

(event `self.Front Collider.OnComponentBeginOverlap`
  (params (OverlappedComponent :type "PrimitiveComponent Object Reference") (OtherActor :type "Actor Object Reference") (OtherComp :type "PrimitiveComponent Object Reference") (OtherBodyIndex :type Integer) (bFromSweep :type Boolean) (SweepResult :type "HitResult Structure (by ref)"))
  (goto _label))

(event `self.Right Collider.OnComponentBeginOverlap`
  (params (OverlappedComponent :type "PrimitiveComponent Object Reference") (OtherActor :type "Actor Object Reference") (OtherComp :type "PrimitiveComponent Object Reference") (OtherBodyIndex :type Integer) (bFromSweep :type Boolean) (SweepResult :type "HitResult Structure (by ref)"))
  (goto _label_2))

(event `self.Left Collider.OnComponentBeginOverlap`
  (params (OverlappedComponent :type "PrimitiveComponent Object Reference") (OtherActor :type "Actor Object Reference") (OtherComp :type "PrimitiveComponent Object Reference") (OtherBodyIndex :type Integer) (bFromSweep :type Boolean) (SweepResult :type "HitResult Structure (by ref)"))
  (goto _label_3))

(fn `UserConstructionScript`)