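; BP_Player2 is a player-controlled pawn with toggled forward movement and axis-driven strafing.
; Accelerate sets a Moving flag and Brake clears it; while set, Tick adds forward movement input and prints the actor location to screen.
; Strafe Right feeds its axis value into sideways movement input, and both directions derive from control rotation yaw only.
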(event `InputAction|Accelerate`
  (params (Key :type "Key Structure"))
  (:`Pressed`
    (set `self.moving` true)))

(event `InputAction|Brake`
  (params (Key :type "Key Structure"))
  (:`Pressed`
    (set `self.moving` false)))

(event `self.ReceiveTick`
  (params (DeltaSeconds :type "Float (single-precision)"))
  (if (`self.moving`)
    (`self.AddMovementInput` (`KismetMathLibrary.GetForwardVector` (`KismetMathLibrary.MakeRotator` 0.0 0.0 (.yaw (`self.GetControlRotation`)))) 20.0)
    (`KismetSystemLibrary.PrintString` (`KismetStringLibrary.Conv_VectorToString` (`self.K2_GetActorLocation`)))))

(event `InputAxis|Strafe Right`
  (params (AxisValue :type "Float (single-precision)"))
  (`self.AddMovementInput` (`KismetMathLibrary.GetRightVector` (`KismetMathLibrary.MakeRotator` 0.0 0.0 (.yaw (`self.GetControlRotation`)))) AxisValue))

(fn `UserConstructionScript`)