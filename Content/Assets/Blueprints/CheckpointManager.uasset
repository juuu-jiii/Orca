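; CheckpointManager tracks lap progress, lap count and lap times for a course of ordered checkpoints.
; Tick accumulates LapTime, while UpdateCheckpoints accepts only the expected next checkpoint number and returns whether to mark it visited.
; Reaching the end of the Checkpoints array records any fastest lap, restarts the timer, increments LapCount and resets all checkpoints and indices.
; Wrong-direction lap reset remains a TODO.
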(event `self.ReceiveBeginPlay`
  (`self.Init`))

(event `self.ReceiveTick`
  (params (DeltaSeconds :type "Float (single-precision)"))
  ;[1 1 1] Update lapTime each frame.
  (set `self.lapTime` (+ DeltaSeconds (`self.lapTime`))))

(fn `CompleteLap`
  (bind _checkpoints (`self.Checkpoints`))
  (`self.UpdateLaptimes`)
  (`/Engine/EditorBlueprintResources/StandardMacros.IncrementInt` (`self.lapCount`) ; Increment lapCount.
    (:`  `
      ;[1 1 1] Reset all checkpoints in the array to unvisited.
      (for _index (range (`KismetArrayLibrary.Array_Length` _checkpoints))
        (`/Game/Assets/Blueprints/Checkpoint.Reset` (`|GetArrayItem` _checkpoints _index)))
      (bind _output_get (set `self.currentCheckpoint` 0)) ; Reset currentCheckpoint and \nnextCheckpoint to their initial \nvalues.
      (set `self.nextCheckpoint` (+ _output_get 1)))))

(fn `Init`
  ;[1 1 1] Initialise with appropriate checkpoint-related data.
  (bind _output_get (set `self.currentCheckpoint` 0))
  (set `self.nextCheckpoint` (+ _output_get 1)))

(fn `UpdateCheckpoints`
  (params (checkpointNumber :type Integer))
  (returns (valid :type Boolean))
  (if (== checkpointNumber (`self.nextCheckpoint`))
    ;[1 1 1] Set currentCheckpoint = nextCheckpoint, increment nextCheckpoint, and then check to
    ; see if the lap has been completed i.e., if nextCheckpoint == checkpoints.Length
    (set `self.currentCheckpoint` (`self.nextCheckpoint`))
    (bind _result (`/Engine/EditorBlueprintResources/StandardMacros.IncrementInt` (`self.nextCheckpoint`))
      (:`  `
        (if (== _result (`KismetArrayLibrary.Array_Length` (`self.Checkpoints`)))
          (`self.CompleteLap`)
          (return false) ; Lap complete.\nDo not mark this\nnode visited, as that\nwill mess with future \nlap completion \ndetection.
          (else
            (return true) ; Lap not complete yet.\nMark this checkpoint\nvisited and continue.
          ))))
    (else
      ;[1 1 1] TODO: reset lap if going in opposite direction and overlapping start/finish line.
      (return false))))

(fn `UpdateLaptimes`
  (if (== (`self.lapCount`) 0)
    (set `self.fastestLap` (`self.lapTime`) :!label _label)
    (elif (< (`self.lapTime`) (`self.fastestLap`))
      (goto _label)
      (else
        _)))
  (set `self.lapTime` 0.0) ; Reset current laptime.
)

(fn `UserConstructionScript`)