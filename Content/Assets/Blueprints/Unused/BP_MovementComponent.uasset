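; Movement component that drives its owning pawn by setting velocity on a physics-simulated box collider root.
; Tick normalises consumed movement input and draws a debug velocity trace.
; A looping fixed-step timer, imitating FixedUpdate, adds input acceleration to the current velocity and writes it back, without clamping speed.
; Steer helpers yaw the pawn by 90 degrees; manual gravity and rotation-lock logic exist but are not wired in.
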(event `self.ReceiveBeginPlay`
  (bind _aspawn (cast `Pawn` (`self.GetOwner`)))
  (bind _output_get (set `self.ParentPawn` _aspawn)) ; Pawn - used later \nto read player input.
  (bind _asbox_collision (cast `BoxComponent` (`Actor.RootComponent` _output_get))) ; Collider
  (set `self.BoxCollider` _asbox_collision)
  (`self.InitPhysics`)
  (`KismetSystemLibrary.K2_SetTimerDelegate` (delegate `FixedTick`) (`self.FixedDeltaTime`) true) ; Works like FixedUpdate, for \nphysics calculations.
)

(event `FixedTick`
  (set `self.Velocity` (`SceneComponent.GetComponentVelocity` (`self.BoxCollider`)))
  (`self.UpdateVelocity` 10.0)
  (`PrimitiveComponent.SetAllPhysicsLinearVelocity` (`self.BoxCollider`) (`self.Velocity`) false) ; Pass the calculated velocity value \nto the Box Collider.
)

(event `self.ReceiveTick`
  (params (DeltaSeconds :type "Float (single-precision)"))
  (bind _parentpawn (`self.ParentPawn`) ; Get ParentPawn\n> right-click\n> convert to validated get
    (:`then`
      (bind _returnvalue (`Pawn.ConsumeMovementInputVector` _parentpawn))
      (set `self.Input` (`KismetMathLibrary.Normal` _returnvalue))
      (`self.ShowVelocity`))
    (:`else`)))

(fn `ApplyGravity`
  (params (GravityEnabled :type Boolean :default false))
  (if GravityEnabled
    (set `self.Velocity` (+ (* (* (`self.GravityDirection`) (`self.GravitationalAcceleration`)) (`self.FixedDeltaTime`)) (`self.Velocity`)))))

(fn `InitPhysics`
  (`self.SetTickGroup` "TG_PostPhysics")
  (`PrimitiveComponent.SetSimulatePhysics` (`self.BoxCollider`) true) ; Enable physics simulation for\ncollisions.
  (`PrimitiveComponent.SetCollisionProfileName` (`self.BoxCollider`) "Pawn" true)
  (`PrimitiveComponent.SetPhysMaterialOverride` (`self.BoxCollider`) "/Game/Assets/Physics/PM_PawnPhysics.PM_PawnPhysics"))

(fn `ShowVelocity`
  (bind _returnvalue (`Actor.K2_GetActorLocation` (`self.ParentPawn`)))
  (`KismetSystemLibrary.LineTraceSingle` :`Start` _returnvalue :`End` (+ _returnvalue (* (`self.Velocity`) 5000.0)) :`TraceChannel` "TraceTypeQuery1" :`DrawDebugType` "ForOneFrame"))

(fn `Steer`
  (params (angle :type "Float (double-precision)"))
  (bind _parentpawn (`self.ParentPawn`))
  (bind (_returnvalue_roll _returnvalue_pitch _returnvalue_yaw) (`KismetMathLibrary.BreakRotator` (`Actor.K2_GetActorRotation` _parentpawn)))
  (`Actor.K2_SetActorRotation` _parentpawn (`KismetMathLibrary.MakeRotator` _returnvalue_roll _returnvalue_pitch (+ angle _returnvalue_yaw)) false))

(fn `SteerLeft`
  (`self.Steer` -90.0))

(fn `SteerRight`
  (`self.Steer` 90.0))

(fn `UpdateVelocity`
  (params (MaxSpeed :type "Float (double-precision)" :default 500.0) (Acceleration :type "Float (double-precision)" :default 10.0))
  (bind _output_get (set `self.Velocity` (+ (* (* (* (`self.Input`) MaxSpeed) Acceleration) (`self.FixedDeltaTime`)) (`self.Velocity`)))) ; Output is accumulated\nin the velocity vector\nvariable.
)