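; Player pawn Blueprint, kept in an Unused folder, that drives itself forward once Accelerate is pressed and stops pushing when Brake is pressed.
; A Moving flag gates forward input on Tick, steering calls to BPMovementComponent and frame-rate-scaled strafing by local offset.
; The Accelerate axis separately adds world-space movement mixed with Steer Right, and R zeroes component velocity.
; Several disconnected movement experiments remain in the graph.
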(event `InputAxis|Accelerate`
  (params (AxisValue :type "Float (single-precision)"))
  (`self.AddMovementInput` (`KismetMathLibrary.MakeVector` AxisValue (`self.GetInputAxisValue`))) ; Pawns have an inbuilt\nAddMovementInput function\nwhich can be used to read \nplayer input inside the \nmovement component.
)

(event `self.ReceiveTick`
  (params (DeltaSeconds :type "Float (single-precision)"))
  (if (`self.moving`)
    (`self.AddMovementInput` (`self.GetActorForwardVector`))))

(event `InputAction|Accelerate`
  (params (Key :type "Key Structure"))
  (:`Pressed`
    (set `self.moving` true)))

(event `InputAction|Brake`
  (params (Key :type "Key Structure"))
  (:`Pressed`
    (set `self.moving` false)))

(event `InputAction|Steer Left`
  (params (Key :type "Key Structure"))
  (:`Pressed`
    (if (`self.moving`)
      (`/Game/Assets/Blueprints/Unused/BP_MovementComponent.SteerLeft` (`self.BP_MovementComponent`)))))

(event `InputAction|Steer Right`
  (params (Key :type "Key Structure"))
  (:`Pressed`
    (if (`self.moving`)
      (`/Game/Assets/Blueprints/Unused/BP_MovementComponent.SteerRight` (`self.BP_MovementComponent`)))))

(event `InputAxis|Strafe Right`
  (params (AxisValue :type "Float (single-precision)"))
  (if (`self.moving`)
    (`self.K2_AddActorLocalOffset` (`KismetMathLibrary.MakeVector` 0.0 (* (* AxisValue (stale `self.ReceiveTick` DeltaSeconds)) 500.0)))))

(event `Key|O`
  (params (Key :type "Key Structure")))

(event `InputAction|Steer Right`
  (params (Key :type "Key Structure")))

(event `Key|P`
  (params (Key :type "Key Structure")))

(event `Key|R`
  (params (Key :type "Key Structure"))
  (:`Pressed`
    (set `/Game/Assets/Blueprints/Unused/BP_MovementComponent.Velocity` (0.0 0.0 0.0) (`self.BP_MovementComponent`))))

(fn `UserConstructionScript`)