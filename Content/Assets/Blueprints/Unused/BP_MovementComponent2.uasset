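; An unused-folder movement component that drives its owning pawn through physics velocity on its root box collider.
; On BeginPlay it caches the pawn and box, sets ticking to post-physics and sets the collision profile to "None".
; Each tick it normalizes consumed movement input, adds scaled acceleration to current velocity and writes it back.
; MaxSpeed only scales acceleration without clamping, and the FixedDeltaTime function it relies on is empty.
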(event `self.ReceiveBeginPlay`
  (bind _aspawn (cast `Pawn` (`self.GetOwner`)))
  (bind _output_get (set `self.Pawn` _aspawn))
  (bind _asbox_collision (cast `BoxComponent` (`Actor.RootComponent` _output_get)))
  (set `self.BoxCollider` _asbox_collision)
  (`self.InitPhysics`))

(event `self.ReceiveTick`
  (params (DeltaSeconds :type "Float (single-precision)"))
  (bind _pawn (`self.Pawn`)
    (:`then`
      (bind _returnvalue (`Pawn.ConsumeMovementInputVector` _pawn))
      (set `self.Input` (`KismetMathLibrary.Normal` _returnvalue)) ; Getting, normalising, then\nsetting the value of input from  \nGetMovementInput
      (set `self.Velocity` (`SceneComponent.GetComponentVelocity` (`self.BoxCollider`))) ; Get and store current velocity
      (`self.UpdateVelocity` 50.0)
      (`PrimitiveComponent.SetAllPhysicsLinearVelocity` (`self.BoxCollider`) (`self.Velocity`) false))
    (:`else`)))

(fn `InitPhysics`
  (`self.SetTickGroup` "TG_PostPhysics")
  (`PrimitiveComponent.SetCollisionProfileName` (`self.BoxCollider`) "None" true))

(fn `UpdateVelocity`
  (params (MaxSpeed :type "Float (double-precision)" :default 50.0) (Acceleration :type "Float (double-precision)" :default 10.0))
  (set `self.Velocity` (+ (* (* (* (`self.Input`) MaxSpeed) Acceleration) (`self.FixedDeltaTime`)) (`self.Velocity`))))