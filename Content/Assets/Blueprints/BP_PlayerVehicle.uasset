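; Player vehicle pawn for a track racer that drives itself forward once accelerated, with strafing and 90-degree snap turns.
; Tick runs a Stopped/Moving/Grinding/Crashed state machine, slowing while grinding and respawning at CheckpointManager's checkpoint after a crash cooldown.
; Tagged collider overlaps set states: front walls crash, boost squares raise speed, side walls grind with sparks on Track1 only.
; Also creates the HUD for crash text and times Niagara tire smoke bursts.
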(event `self.ReceiveBeginPlay`
  ;[1 1 1] Instantiates the HUD Blueprint and displays it on the screen.
  (bind _returnvalue (`|CreateWidget` "/Game/Assets/UI/WG_HUD.WG_HUD_C"))
  (bind _output_get (set `self.hud` _returnvalue))
  (`UserWidget.AddToViewport` _output_get 0)
  (`WidgetBlueprintLibrary.SetInputMode_GameOnly` (`GameplayStatics.GetPlayerController` 0)) ; Turn off the cursor and set the input \nfor the player to Game Only.
)

(event `InputAction|Accelerate`
  (params (Key :type "Key Structure"))
  ;[1 1 1] Player movement
  ;;[1 1 1] Play smoke animation if vehicle accelerates from a standstill.
  (:`Pressed`
    (if (and (not (`|EnumEquality` (`self.state`) "NewEnumerator1")) (not (`|EnumEquality` (`self.state`) "NewEnumerator2")))
      (set `self.state` "NewEnumerator1")
      (`self.PlayTireSmoke`))))

(event `InputAction|Brake`
  (params (Key :type "Key Structure"))
  ;[1 1 1] Player movement
  ;;[1 1 1] Play smoke animation if vehicle decelerates to a halt.
  (:`Pressed`
    (if (not (`|EnumEquality` (`self.state`) "NewEnumerator0"))
      (set `self.state` "NewEnumerator0")
      (`self.PlayTireSmoke`))))

(event `InputAxis|Strafe Right`
  (params (AxisValue :type "Float (single-precision)"))
  (bind _state (`self.state`))
  ;[1 1 1] Player movement
  ;;[1 1 1] Strafe L/R
  (if (or (`|EnumEquality` _state "NewEnumerator1") (`|EnumEquality` _state "NewEnumerator2"))
    (`self.AddMovementInput` (+ (* (`self.GetActorRightVector`) AxisValue) (`self.GetActorForwardVector`)) 10000.0)))

(event `self.ReceiveTick`
  (params (DeltaSeconds :type "Float (single-precision)"))
  (bind _checkpointmanager (`self.checkpointManager`))
  ;[1 1 1] Player FSM
  (`self.HandleTireSmoke` DeltaSeconds)
  (switch `/Game/Assets/Blueprints/Enums/VehicleStates` (`self.state`)
    (:`NewEnumerator1`
      ;;[1 1 1] Moving - travel at regular speed.
      (set `FloatingPawnMovement.MaxSpeed` (`self.speed`) (`self.FloatingPawnMovement`))
      (`self.AddMovementInput` (`self.GetActorForwardVector`)))
    (:`NewEnumerator2`
      ;;[1 1 1] Grinding - travel at reduced speed.
      (set `FloatingPawnMovement.MaxSpeed` (* (`self.speed`) (`self.speedReductionFactor`)) (`self.FloatingPawnMovement`))
      (`self.AddMovementInput` (`self.GetActorForwardVector`)))
    (:`NewEnumerator3`
      ;;[1 1 1] Crashed - 1 second cooldown, then reset vehicle.
      (if (< (`self.crashTimer`) 1.0)
        (set `self.crashTimer` (+ (`self.crashTimer`) DeltaSeconds))
        (else
          (set `self.state` "NewEnumerator0")
          (`/Game/Assets/UI/WG_HUD.SetAlphaCrash` (`self.hud`) 0.0) ; Hide CRASH! text.
          (set `self.crashTimer` 0.0)
          (`self.K2_SetActorLocation` (`/Game/Assets/Blueprints/CheckpointManager.currentCheckpointLocation` _checkpointmanager)) ; Reset car to last checkpoint location.
          (`self.K2_SetActorRotation` (`KismetMathLibrary.Conv_VectorToRotator` (`/Game/Assets/Blueprints/CheckpointManager.currentCheckpointForwardVector` _checkpointmanager))) ; Point car in the correct direction i.e., \nalong the last checkpoint's forward \nvector.
          (`self.EnableInput` null))))))

(event `InputAction|Steer Left`
  (params (Key :type "Key Structure"))
  (bind (_returnvalue_roll _returnvalue_pitch _returnvalue_yaw) (`KismetMathLibrary.BreakRotator` (`self.K2_GetActorRotation`)))
  (bind _state (`self.state`))
  ;[1 1 1] Player movement
  ;;[1 1 1] Steer L/R
  (:`Pressed`
    (if (or (`|EnumEquality` _state "NewEnumerator1") (`|EnumEquality` _state "NewEnumerator2"))
      (`self.K2_SetActorRotation` (`KismetMathLibrary.MakeRotator` 0.0 0.0 (+ -90.0 _returnvalue_yaw)))
      (`self.PlayTireSmoke`))))

(event `InputAction|Steer Right`
  (params (Key :type "Key Structure"))
  (bind (_returnvalue_roll _returnvalue_pitch _returnvalue_yaw) (`KismetMathLibrary.BreakRotator` (`self.K2_GetActorRotation`)))
  (bind _state (`self.state`))
  ;[1 1 1] Player movement
  ;;[1 1 1] Steer L/R
  (:`Pressed`
    (if (or (`|EnumEquality` _state "NewEnumerator1") (`|EnumEquality` _state "NewEnumerator2"))
      (`self.K2_SetActorRotation` (`KismetMathLibrary.MakeRotator` 0.0 0.0 (+ 90.0 _returnvalue_yaw)))
      (`self.PlayTireSmoke`))))

(event `self.Front Collider.OnComponentBeginOverlap`
  (params (OverlappedComponent :type "PrimitiveComponent Object Reference") (OtherActor :type "Actor Object Reference") (OtherComp :type "PrimitiveComponent Object Reference") (OtherBodyIndex :type Integer) (bFromSweep :type Boolean) (SweepResult :type "HitResult Structure (by ref)"))
  ;[1 1 1] Collision handling
  (if (`self.ActorHasTag` OtherActor "Wall")
    (set `self.state` "NewEnumerator3")
    (`/Game/Assets/UI/WG_HUD.SetAlphaCrash` (`self.hud`) 1.0) ; Show CRASH! text.
    (`self.DisableInput` null) ; During crash timer\ncountdown, disallow \nplayer input.
    (elif (`self.ActorHasTag` OtherActor "Boost Square")
      (set `self.speed` (* (`self.speed`) 1.05)))))

(event `Key|BackSpace`
  (params (Key :type "Key Structure"))
  ;[1 0.251 0] Backspace to go back to main
  (:`Pressed`
    (`GameplayStatics.OpenLevelBySoftObjectPtr` "/Game/Assets/Levels/MainMenu.MainMenu")
    (`Widget.RemoveFromParent` (`self.hud`))))

(event `self.Left Collider.OnComponentBeginOverlap`
  (params (OverlappedComponent :type "PrimitiveComponent Object Reference") (OtherActor :type "Actor Object Reference") (OtherComp :type "PrimitiveComponent Object Reference") (OtherBodyIndex :type Integer) (bFromSweep :type Boolean) (SweepResult :type "HitResult Structure (by ref)"))
  ;[1 1 1] Collision handling
  ;;[1 1 1] Hit on the side= grinding
  ;[1 0.251 0] If name != Track1 disable grinding
  (bind _returnvalue (`GameplayStatics.GetCurrentLevelName` true))
  (if (`KismetStringLibrary.EqualEqual_StrStr` "Track1" _returnvalue)
    (if (and (`self.ActorHasTag` OtherActor "Wall") (`|EnumInequality` "NewEnumerator3" (`self.state`)))
      (set `self.state` "NewEnumerator2")
      (`ActorComponent.Activate` (`self.SparksLeft`) false))))

(event `self.Right Collider.OnComponentBeginOverlap`
  (params (OverlappedComponent :type "PrimitiveComponent Object Reference") (OtherActor :type "Actor Object Reference") (OtherComp :type "PrimitiveComponent Object Reference") (OtherBodyIndex :type Integer) (bFromSweep :type Boolean) (SweepResult :type "HitResult Structure (by ref)"))
  ;[1 1 1] Collision handling
  ;;[1 1 1] Hit on the side= grinding
  ;[1 0.251 0] If name != Track1 disable grinding
  (bind _returnvalue (`GameplayStatics.GetCurrentLevelName` true))
  (if (`KismetStringLibrary.EqualEqual_StrStr` "Track1" _returnvalue)
    (if (and (`self.ActorHasTag` OtherActor "Wall") (`|EnumInequality` "NewEnumerator3" (`self.state`)))
      (set `self.state` "NewEnumerator2")
      (`ActorComponent.Activate` (`self.SparksRight`) false))))

(event `self.Left Collider.OnComponentEndOverlap`
  (params (OverlappedComponent :type "PrimitiveComponent Object Reference") (OtherActor :type "Actor Object Reference") (OtherComp :type "PrimitiveComponent Object Reference") (OtherBodyIndex :type Integer))
  ;[1 1 1] Collision handling
  ;;[1 1 1] Exit overlap = transition grinding --> moving
  ;[1 0.251 0] If name != Track1 disable grinding
  (bind _returnvalue (`GameplayStatics.GetCurrentLevelName` true))
  (if (`KismetStringLibrary.EqualEqual_StrStr` "Track1" _returnvalue)
    (if (and (`self.ActorHasTag` OtherActor "Wall") (`|EnumInequality` "NewEnumerator3" (`self.state`)))
      (set `self.state` "NewEnumerator1")
      (`ActorComponent.Deactivate` (`self.SparksLeft`)))))

(event `self.Right Collider.OnComponentEndOverlap`
  (params (OverlappedComponent :type "PrimitiveComponent Object Reference") (OtherActor :type "Actor Object Reference") (OtherComp :type "PrimitiveComponent Object Reference") (OtherBodyIndex :type Integer))
  ;[1 1 1] Collision handling
  ;;[1 1 1] Exit overlap = transition grinding --> moving
  ;[1 0.251 0] If name != Track1 disable grinding
  (bind _returnvalue (`GameplayStatics.GetCurrentLevelName` true))
  (if (`KismetStringLibrary.EqualEqual_StrStr` "Track1" _returnvalue)
    (if (and (`self.ActorHasTag` OtherActor "Wall") (`|EnumInequality` "NewEnumerator3" (`self.state`)))
      (set `self.state` "NewEnumerator1")
      (`ActorComponent.Deactivate` (`self.SparksRight`)))))

(fn `HandleTireSmoke`
  (params (deltaSeconds :type "Float (double-precision)"))
  (if (`self.tiresSmoking`)
    (set `self.currentSmokeDuration` (+ deltaSeconds (`self.currentSmokeDuration`)))
    (if (>= (`self.currentSmokeDuration`) (`self.smokeDuration`))
      (`self.StopTireSmoke`))))

(fn `PlayTireSmoke`
  (`NiagaraComponent.SetVariableFloat` (`self.Tire Smoke`) "User.spawnRate" 25.0)
  (set `self.tiresSmoking` true)
  (set `self.currentSmokeDuration` 0.0))

(fn `StopTireSmoke`
  (`NiagaraComponent.SetVariableFloat` (`self.Tire Smoke`) "User.spawnRate" 0.0)
  (set `self.tiresSmoking` false)
  (set `self.currentSmokeDuration` 0.0))

(fn `UserConstructionScript`)