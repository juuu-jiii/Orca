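; Checkpoint actor that registers with a checkpoint manager when the player passes through its box trigger.
; On overlap by an actor tagged Player, an unvisited checkpoint passes itself to CheckpointManager.UpdateCheckpoints and stores the result as its Visited flag, so the manager decides whether the visit counts.
; A Reset function clears the flag to return the checkpoint to its unvisited state.
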(event `self.Box.OnComponentBeginOverlap`
  (params (OverlappedComponent :type "PrimitiveComponent Object Reference") (OtherActor :type "Actor Object Reference") (OtherComp :type "PrimitiveComponent Object Reference") (OtherBodyIndex :type Integer) (bFromSweep :type Boolean) (SweepResult :type "HitResult Structure (by ref)"))
  ;[1 1 1] Only bother if overlapping with the player and if this checkpoint has not been visited yet.
  (if (and (`self.ActorHasTag` OtherActor "Player") (not (`self.visited`)))
    (bind _valid (`/Game/Assets/Blueprints/CheckpointManager.Update Checkpoints` (`self.checkpointManager`) self))
    (set `self.visited` _valid)))

(fn `Reset`
  ;[1 1 1] Return this checkpoint to its original, unvisited state.
  (set `self.visited` false))

(fn `UserConstructionScript`)